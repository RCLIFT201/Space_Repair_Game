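; BP_PlayerBase is a player base class providing mouse look and gaze-based interaction with BP_InteractiveBase objects.
; Mouse axes drive controller yaw and pitch, scaled by frame time and per-axis speed.
; BasicGaze line-traces forward from the camera and activates a newly focused interactive once, clearing focus otherwise.
; Tick is empty and the event graph's BasicGaze call is disconnected, so this graph never triggers the gaze check.
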(event `self.ReceiveTick`
  (params (DeltaSeconds :type "Float (single-precision)")))

(event `InputAxisKey|MouseX`
  (params (AxisValue :type "Float (single-precision)"))
  (`self.AddControllerYawInput` (* (* AxisValue (`GameplayStatics.GetWorldDeltaSeconds`)) (`self.Mouse Speed X`))))

(event `InputAxisKey|MouseY`
  (params (AxisValue :type "Float (single-precision)"))
  (`self.AddControllerPitchInput` (* (* AxisValue (`GameplayStatics.GetWorldDeltaSeconds`)) (`self.Mouse Speed Y`))))

(fn `BasicGaze`
  (bind (_bblockinghit _binitialoverlap _time _distance _location _impactpoint _normal _impactnormal _physmat _hitactor) (`GameplayStatics.BreakHitResult` (`self.LineTraceForward`)))
  (if _bblockinghit
    (bind _asbp_interactive_base (cast `/Game/GGJ/Blueprints/Interactions/BP_InteractiveBase` _hitactor)
      (:`then`
        (set `self.InteractiveObject` _asbp_interactive_base)
        (if (not (== (`self.InteractiveObject`) (`self.FocusedObject`)))
          (set `self.FocusedObject` (`self.InteractiveObject`))
          (`self.Interact`)))
      (:`CastFailed`
        (set `self.InteractiveObject` null :!label _label)
        (set `self.FocusedObject` null)))
    (else
      (goto _label))))

(fn `Interact`
  (bind _interactiveobject (`self.InteractiveObject`))
  (`/Engine/EditorBlueprintResources/StandardMacros.IsValid` _interactiveobject
    (:`Is Valid`
      (`/Game/GGJ/Blueprints/Interactions/BP_InteractiveBase.Activate` _interactiveobject))))

(fn `LineTraceForward`
  (returns (OutHit :type "HitResult Structure"))
  (bind _camera (`self.Camera`))
  (bind _returnvalue (`SceneComponent.K2_GetComponentLocation` _camera))
  (bind _outhit (`KismetSystemLibrary.LineTraceSingle` _returnvalue (+ _returnvalue (* (`KismetMathLibrary.GetForwardVector` (`SceneComponent.K2_GetComponentRotation` _camera)) 15000.0)) "TraceTypeQuery1"))
  (return _outhit))

(fn `UserConstructionScript`)