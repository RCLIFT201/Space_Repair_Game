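; Asteroid actor that takes damage from first-person projectiles and is destroyed when its health runs out.
; Each projectile hit on the static mesh subtracts a fixed amount from Health.
; A world-space widget rotates every tick to face the player character.
; BeginPlay casts that widget to HealthBar but sets its Owner to None, so the bar receives no reference to the asteroid.
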(event `self.ReceiveBeginPlay`
  (bind _ashealth_bar (cast `/Game/Prefabs/HealthBar` (`WidgetComponent.GetUserWidgetObject` (`self.Widget`))))
  (set `/Game/Prefabs/HealthBar.Owner` null self _ashealth_bar))

(event `self.ReceiveTick`
  (params (DeltaSeconds :type "Float (single-precision)"))
  (bind _widget (`self.Widget`))
  (`SceneComponent.K2_SetWorldRotation` _widget (`KismetMathLibrary.FindLookAtRotation` (`SceneComponent.K2_GetComponentLocation` _widget) (`self.K2_GetActorLocation` (`GameplayStatics.GetPlayerCharacter` 0))) false false))

(event `self.StaticMesh.OnComponentHit`
  (params (HitComponent :type "PrimitiveComponent Object Reference") (OtherActor :type "Actor Object Reference") (OtherComp :type "PrimitiveComponent Object Reference") (NormalImpulse :type "Vector Structure") (Hit :type "HitResult Structure (by ref)"))
  (cast `/Game/FirstPersonBP/Blueprints/FirstPersonProjectile` OtherActor)
  (bind _output_get (set `self.Health` (- (`self.Health`) 10.0)))
  (if (<= _output_get 0.0)
    (`self.K2_DestroyActor`)))

(fn `UserConstructionScript`)